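; Enemy character for the third-person shooter that attacks the player in range and dies from any damage or a Bullet-tagged capsule overlap check.
; Tick polls player distance, applying damage after a short delay; AB_Enemy receives animation states.
; Death tweens a runtime-material dither mask, then hides and disables the actor instead of destroying it.
; Alive, called on BeginPlay and Spawning, starts BP_EnemyAI's behavior tree and restores the mask.
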(event OnComponentBeginOverlap(CapsuleComponent)
  (params (OverlappedComponent :type Primitive%20Component%20Object%20Reference) (OtherActor :type Actor%20Object%20Reference) (OtherComp :type Primitive%20Component%20Object%20Reference) (OtherBodyIndex :type Integer) (bFromSweep :type Boolean) (SweepResult :type Hit%20Result%20Structure%20%28by%20ref%29))
  (if (Actor|ActorHasTag "Bullet")
    (CallFunction|Die)
    (Utilities|FlowControl|Delay 3.0)
    (Rendering|SetActorHiddenInGame true)
    (Collision|SetActorEnableCollision false)
    (Actor|Tick|SetActorTickEnabled false)))

(event Custom|Die
  ;[0.15 0.15 0.15 0.5] Die
  (bind _asab_enemy (Utilities|Casting|CastToAB_Enemy (Components|SkeletalMesh|GetAnimInstance (Variables|Character|GetMesh))))
  (Variables|/Game/TPShooter/Animations/AB_Enemy.AB_Enemy_C|SetEnemyAnimState _asab_enemy "NewEnumerator3")
  (Variables|Default|SetcanAttack false)
  (Utilities|FlowControl|Delay 2.0)
  (CallFunction|Dither))

(event Custom|Attack
  ;[0.15 0.15 0.15 0.5] Attack
  (if (Variables|Default|GetcanAttack)
    (if (Variables|Default|GetisAttacking)
      (bind _asab_enemy (Utilities|Casting|CastToAB_Enemy (Components|SkeletalMesh|GetAnimInstance (Variables|Character|GetMesh))))
      (Variables|/Game/TPShooter/Animations/AB_Enemy.AB_Enemy_C|SetEnemyAnimState _asab_enemy "NewEnumerator2")
      (Game|Damage|ApplyDamage (Game|GetPlayerCharacter 0) (Variables|Default|GetAttackDamage) (Pawn|GetController) self)
      (Variables|Default|SetisAttacking false)
      (CallFunction|BuscaAtacar))))

(event Custom|Alive
  (bind _asbp_enemy_ai (Utilities|Casting|CastToBP_EnemyAI (Pawn|GetController)))
  ;[0.15 0.15 0.15 0.5] Alive
  (AI|RunBehaviorTree _asbp_enemy_ai)
  (bind _asab_enemy (Utilities|Casting|CastToAB_Enemy (Components|SkeletalMesh|GetAnimInstance (Variables|Character|GetMesh))))
  (Variables|/Game/TPShooter/Animations/AB_Enemy.AB_Enemy_C|SetEnemyAnimState _asab_enemy "NewEnumerator0")
  (Utilities|FlowControl|Delay 2.0)
  (Rendering|Material|SetScalarParameterValue (Variables|/Game/TPShooter/Blueprints/BP_RuntimeMat.BP_RuntimeMat_C|GetRuntimeMaterials (Variables|Default|GetBP_RuntimeMat)) (Variables|Default|GetDitherMask) 1.0 :!class /Script/Engine.MaterialInstanceDynamic)
  (Variables|Default|SetDitherActive false))

(event Custom|Busca%20atacar
  ;[0.15 0.15 0.15 0.5] Busca Atacar
  (if (<= (Transformation|GetDistanceTo (Game|GetPlayerCharacter 0)) (Variables|Default|GetAttackRange))
    (Variables|Default|SetisAttacking true)
    (Utilities|FlowControl|Delay 0.5)
    (CallFunction|Attack)))

(event Custom|Dither
  (bind _bp_runtimemat (Variables|Default|GetBP_RuntimeMat))
  (bind _runtimematerials (Variables|/Game/TPShooter/Blueprints/BP_RuntimeMat.BP_RuntimeMat_C|GetRuntimeMaterials _bp_runtimemat))
  ;[0.15 0.15 0.15 0.5] Dither
  (if (not (Variables|Default|GetDitherActive))
    (bind _returnvalue (Rendering|Material|GetScalarParameterValue _runtimematerials (Variables|Default|GetDitherMask) :!class /Script/Engine.MaterialInstanceDynamic))
    (bind _value (|TweenFloat _returnvalue 0.0 2.0 "InOutQuad")
      (:ApplyEasing
        (Rendering|Material|SetScalarParameterValue _runtimematerials (Variables|Default|GetDitherMask) _value :!class /Script/Engine.MaterialInstanceDynamic)
        (Variables|Default|SetDitherActive true)))))

(event EventBeginPlay
  (bind _bp_runtimemat (Variables|Default|GetBP_RuntimeMat))
  (|CallParentFunction)
  (Default|CreateRuntimeMaterials _bp_runtimemat)
  (Default|ApplyRuntimeMaterial _bp_runtimemat (Utilities|Array|MakeArray (Variables|Character|GetMesh)))
  (CallFunction|Alive)
  (Variables|Default|SetcanAttack true))

(event Game|Damage|EventAnyDamage
  (params (Damage :type Float%20%28single-precision%29) (DamageType :type Damage%20Type%20Object%20Reference) (InstigatedBy :type Controller%20Object%20Reference) (DamageCauser :type Actor%20Object%20Reference))
  (CallFunction|Die)
  (Utilities|FlowControl|Delay 3.0)
  (Rendering|SetActorHiddenInGame true)
  (Collision|SetActorEnableCollision false)
  (Actor|Tick|SetActorTickEnabled false))

(event EventTick
  (params (DeltaSeconds :type Float%20%28single-precision%29))
  (|CallParentFunction DeltaSeconds)
  (CallFunction|BuscaAtacar))

(event EventSpawning
  (CallFunction|Alive))

(fn ConstructionScript
  (|CallParentFunction))
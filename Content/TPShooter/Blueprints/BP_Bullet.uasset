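; BP_Bullet is a projectile actor for the third-person shooter that is hidden, rather than destroyed, when spent.
; OnSpawn re-binds and enables its ProjectileMovement on the collision component, launching it along player 0's camera forward at ProjectileSpeed.
; A component hit hides the bullet and stops its movement.
; The LifeTime event hides it after a given delay but leaves movement running.
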(event OnComponentHit(Colision)
  (params (HitComponent :type Primitive%20Component%20Object%20Reference) (OtherActor :type Actor%20Object%20Reference) (OtherComp :type Primitive%20Component%20Object%20Reference) (NormalImpulse :type Vector :default "0, 0, 0") (Hit :type Hit%20Result%20Structure%20%28by%20ref%29))
  (Class|ActorUtilities|ToggleActorHidden self true)
  (Components|Movement|StopMovementImmediately (Variables|Default|GetProjectileMovement)))

(event EventBeginPlay)

(event Collision|EventActorBeginOverlap
  (params (OtherActor :type Actor%20Object%20Reference)))

(event EventTick
  (params (DeltaSeconds :type Float%20%28single-precision%29)))

(event EventOnSpawn
  (params (instigator :type Actor%20Object%20Reference))
  (bind _projectilemovement (Variables|Default|GetProjectileMovement))
  ;[0.15 0.15 0.15 0.5] Spawn de la bala
  (Components|Movement|SetUpdatedComponent (Variables|Default|GetProjectileMovement) (Variables|Default|GetColision))
  (Variables|/Script/Engine.ProjectileMovementComponent|SetbSimulationEnabled _projectilemovement true)
  (Variables|/Script/Engine.MovementComponent|SetVelocity _projectilemovement (* (Math|Vector|GetForwardVector (Camera|GetCameraRotation (Variables|/Script/Engine.PlayerController|GetPlayerCameraManager (Game|GetPlayerController 0)))) (Variables|Default|GetprojectileSpeed))))

(event EventLifeTime
  (params (time :type Float%20%28single-precision%29))
  ;[0.15 0.15 0.15 0.5] Tiempo de vida de la bala
  (Utilities|FlowControl|Delay time)
  (Class|ActorUtilities|ToggleActorHidden self true))

(fn ConstructionScript)
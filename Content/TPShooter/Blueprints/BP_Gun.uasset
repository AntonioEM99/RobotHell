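; BP_Gun is the TPShooter gun actor that fires bullets from a shared actor pool instead of spawning them.
; On BeginPlay it caches the bullet pool from the game mode.
; HandleShoot teleports a pooled bullet to the muzzle spawn point with its rotation, then messages it the gun's owner and a lifetime.
; A separate Shoot function does the same with a pool validity check, but without setting rotation or teleporting.
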(event EventBeginPlay
  (bind _asbp_tpshooter_game_mode (Utilities|Casting|CastToBP_TPShooterGameMode (Game|GetGameMode)))
  (Variables|Default|SetActor%20Pool%20Bullet (Variables|/Game/TPShooter/Blueprints/BP_TPShooterGameMode.BP_TPShooterGameMode_C|GetActorPoolBullet _asbp_tpshooter_game_mode)))

(event Collision|EventActorBeginOverlap
  (params (OtherActor :type Actor%20Object%20Reference)))

(event EventTick
  (params (DeltaSeconds :type Float%20%28single-precision%29)))

(event EventHandleShoot
  ;[0.15 0.15 0.15 0.5] Shoot
  (Utilities|Casting|CastToBP_TPShooterGameMode (Game|GetGameMode))
  (bind _returnvalue (Class|ActorPool|GetActorfromPool (Variables|Default|GetActor%20Pool%20Bullet)))
  (Transformation|SetActorLocation _returnvalue (Transformation|GetWorldLocation (Variables|Default|GetProyectileSpawnPoint)) false true)
  (Transformation|SetActorRotation _returnvalue (Transformation|GetWorldRotation (Variables|Default|GetProyectileSpawnPoint)))
  (Class|IPooled|OnSpawn(Message) _returnvalue (Components|GetOwner))
  (Class|IPooled|LifeTime(Message) _returnvalue 3.0))

(fn ConstructionScript)

(fn Shoot
  (bind _actor_pool_bullet (Variables|Default|GetActor%20Pool%20Bullet)
    (:then
      (bind _returnvalue (Class|ActorPool|GetActorfromPool _actor_pool_bullet))
      (Transformation|SetActorLocation _returnvalue (Transformation|GetWorldLocation (Variables|Default|GetProyectileSpawnPoint)) false false)
      (Class|IPooled|OnSpawn(Message) _returnvalue (Components|GetOwner))
      (Class|IPooled|LifeTime(Message) _returnvalue 3.0))
    (:else)))
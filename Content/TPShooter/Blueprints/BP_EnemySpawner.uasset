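; Enemy spawner actor for the third-person shooter that brings pooled enemies into play at its spawn point.
; A looping three-second timer started on BeginPlay requests an actor from the game mode's enemy actor pool.
; A valid actor is moved to the spawn point, unhidden and given collision, reusing instances instead of spawning new ones.
; An invalid result only prints a debug message.
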(event Custom|Spawn%20Enemy
  (bind _asbp_tpshooter_game_mode (Utilities|Casting|CastToBP_TPShooterGameMode (Game|GetGameMode)))
  (bind _returnvalue (Class|ActorPool|GetActorfromPool (Variables|/Game/TPShooter/Blueprints/BP_TPShooterGameMode.BP_TPShooterGameMode_C|GetActorPoolEnemies _asbp_tpshooter_game_mode)))
  (Utilities|IsValid _returnvalue
    (:Is%20Valid
      (Transformation|SetActorLocation _returnvalue (Transformation|GetWorldLocation (Variables|Default|GetSpawnPoint)) false false)
      (Rendering|SetActorHiddenInGame _returnvalue false)
      (Collision|SetActorEnableCollision _returnvalue true))
    (:Is%20Not%20Valid
      (Development|PrintString "No valido"))))

(event EventBeginPlay
  (Utilities|Time|SetTimerbyEvent (delegate Custom|Spawn%20Enemy) 3.0 true))

(event Collision|EventActorBeginOverlap
  (params (OtherActor :type Actor%20Object%20Reference)))

(event EventTick
  (params (DeltaSeconds :type Float%20%28single-precision%29)))

(fn ConstructionScript)
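; BP_DecalScorch is a scorch mark decal actor that fades out after a requested lifetime.
; On BeginPlay it creates a dynamic material instance from its decal and stores it as RuntimeMat.
; The LifeTime event starts the decal fade after the given time, then hides the actor instead of destroying it once the fade completes.
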(event EventBeginPlay
  (bind _returnvalue (Rendering|Material|CreateDynamicMaterialInstance (Variables|Decal|GetDecal) :!class /Script/Engine.DecalComponent))
  (Variables|Default|SetRuntimeMat _returnvalue))

(event EventTick
  (params (DeltaSeconds :type Float%20%28single-precision%29)))

(event EventLifeTime
  (params (time :type Float%20%28single-precision%29))
  (bind _fadeduration (Variables|Default|GetFadeDuration))
  (bind _decal (Variables|Decal|GetDecal)
    (:then
      (Rendering|Components|Decal|SetFadeOut _decal time _fadeduration false)
      (Utilities|FlowControl|Delay (+ time _fadeduration))
      (Class|ActorUtilities|ToggleActorHidden self true))
    (:else)))

(fn ConstructionScript)